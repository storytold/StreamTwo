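; Player controller that acts as a level-select shortcut for a set of Zelda-themed levels.
; Number keys 1 through 7 each open their matching level directly by absolute name when pressed.
; The rest of the graph is empty, with BeginPlay, Tick and the construction script doing nothing.
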(event `Key|One`
  (params (Key :type "Key Structure"))
  ;[0.09772 1 0.6124] Level Teleportation
  (:`Pressed`
    (`GameplayStatics.OpenLevel` "/Game/Zelda/level1")))

(event `Key|Two`
  (params (Key :type "Key Structure"))
  ;[0.09772 1 0.6124] Level Teleportation
  (:`Pressed`
    (`GameplayStatics.OpenLevel` "/Game/Zelda/level2")))

(event `Key|Three`
  (params (Key :type "Key Structure"))
  ;[0.09772 1 0.6124] Level Teleportation
  (:`Pressed`
    (`GameplayStatics.OpenLevel` "/Game/Zelda/level3")))

(event `Key|Four`
  (params (Key :type "Key Structure"))
  ;[0.09772 1 0.6124] Level Teleportation
  (:`Pressed`
    (`GameplayStatics.OpenLevel` "/Game/Zelda/level_04")))

(event `Key|Five`
  (params (Key :type "Key Structure"))
  ;[0.09772 1 0.6124] Level Teleportation
  (:`Pressed`
    (`GameplayStatics.OpenLevel` "/Game/Zelda/level_05")))

(event `Key|Six`
  (params (Key :type "Key Structure"))
  ;[0.09772 1 0.6124] Level Teleportation
  (:`Pressed`
    (`GameplayStatics.OpenLevel` "/Game/Zelda/level_06")))

(event `Key|Seven`
  (params (Key :type "Key Structure"))
  ;[0.09772 1 0.6124] Level Teleportation
  (:`Pressed`
    (`GameplayStatics.OpenLevel` "/Game/Zelda/level_07")))

(fn `UserConstructionScript`)